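; Gameplay ability that unequips the hero's axe and returns it to the back socket.
; On activation it plays the unequip montage, clears the equipped weapon tag, and waits for the Player.Event.Unequip.Axe gameplay event.
; That event attaches the axe to the back socket, then unlinks its anim layer, removes its input mapping context and revokes its granted abilities.
; The ability ends when the montage completes, blends out, or is interrupted or cancelled.
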(event Ability|EventActivateAbility
  (|PlayMontageandWaitProxy "None" "/Game/PlayerCharacters/Montages/AM_Hero_Axe_Unequip.AM_Hero_Axe_Unequip" 1.0 "None" true 1.0 0.0 false
    (:then
      (Variables|/Script/WarriorRPG.PawnCombatComponent|SetCurrentEquippedWeaponTag (Class|WarriorHeroGameplayAbility|GetHeroCombatComponentfromActorInfo) "")
      (Ability|Tasks|WaitGameplayEvent "(TagName=\"Player.Event.Unequip.Axe\")" 0
        (:EventReceived
          (Transformation|AttachComponentToComponent (Class|PawnCombatComponent|GetCharacterCarriedWeaponbyTag (Class|WarriorHeroGameplayAbility|GetHeroCombatComponentfromActorInfo) "(TagName=\"Player.Weapon.Axe\")") (Class|GameplayAbility|GetOwningComponentfromActorInfo) "AxeBackSocket" "SnapToTarget" "KeepRelative" "KeepWorld" true)
          (CallFunction|HandleUnequipWeapon (Class|HeroCombatComponent|GetHeroCarriedWeaponbyTag (Class|WarriorHeroGameplayAbility|GetHeroCombatComponentfromActorInfo) "(TagName=\"Player.Weapon.Axe\")")))))
    (:OnCompleted
      (Ability|EndAbility :!label _label))
    (:OnBlendOut
      (goto _label))
    (:OnInterrupted
      (goto _label))
    (:OnCancelled
      (goto _label))))

(event Ability|EventOnEndAbility
  (params (bWasCancelled :type Boolean)))

(fn HandleUnequipWeapon
  (params (InHeroWeapon :type Warrior%20Hero%20Weapon%20Object%20Reference))
  (LocalVariables|SetCatchedHeroWeaponData (Variables|/Script/WarriorRPG.WarriorHeroWeapon|GetHeroWeaponData InHeroWeapon))
  (Utilities|FlowControl|Sequence
    (:then_0
      (CallFunction|FUnlinkAnimLayer (LocalVariables|GetCatchedHeroWeaponData)))
    (:then_1
      (CallFunction|FRemoveInputMapping (LocalVariables|GetCatchedHeroWeaponData)))
    (:then_2
      (CallFunction|FRemoveGrantedWeaponAbilities (Class|WarriorHeroWeapon|GetGrantedAbilitySpecHandles InHeroWeapon)))))

(fn FUnlinkAnimLayer
  (params (InWeaponData :type Warrior%20Hero%20Weapon%20Data%20Structure))
  (Class|SkeletalMeshComponent|UnlinkAnimClassLayers (Class|GameplayAbility|GetOwningComponentfromActorInfo) (.WeaponAnimLayerToLink (Utilities|Struct|BreakWarriorHeroWeaponData InWeaponData))))

(fn FRemoveGrantedWeaponAbilities
  (params (InSpecHandles :type Array%20of%20Gameplay%20Ability%20Spec%20Handle%20Structures))
  (Class|WarriorAbilitySystemComponent|RemoveGrantedHeroWeaponAbilities (Class|WarriorGameplayAbility|GetWarriorAbilitySystemComponentfromActorInfo) InSpecHandles))

(fn FRemoveInputMapping
  (params (InWeaponData :type Warrior%20Hero%20Weapon%20Data%20Structure))
  (Input|RemoveMappingContext (PlayerController|LocalPlayerSubsystems|GetEnhancedInputLocalPlayerSubsystem (Class|WarriorHeroGameplayAbility|GetHeroControllerfromActorInfo)) (.WeaponInputMappingContext (Utilities|Struct|BreakWarriorHeroWeaponData InWeaponData)) "(bIgnoreAllPressedKeysUntilRelease=True,bForceImmediately=False,bNotifyUserSettings=False)"))